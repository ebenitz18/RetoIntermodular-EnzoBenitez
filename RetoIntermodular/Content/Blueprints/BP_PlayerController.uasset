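; Player controller that sets up the local player's interface and relays input and perspective events.
; On BeginPlay, the local controller checks game state, then retries every 0.2 seconds until PlayerState exists before creating WBP_GeneralInterface and rebuilding its score list.
; ExecuteAction fires the OnInputReceived dispatcher.
; RPCServerInput destroys a given actor after a delay, and MCReturnToThirdPerson switches player 0's character back to third person.
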(event Custom|CheckReady
  (Utilities|IsValid (Game|GetGameState)
    (:Is%20Valid
      (Utilities|IsValid (Game|GetPlayerState 0)
        (:Is%20Valid
          (bind _returnvalue (UserInterface|CreateWidget "/Game/Blueprints/WBP_GeneralInterface.WBP_GeneralInterface_C"))
          (UserInterface|Viewport|AddtoViewport _returnvalue 0)
          (Default|RebuildScoreList _returnvalue))
        (:Is%20Not%20Valid
          (Utilities|FlowControl|Delay 0.2)
          (CallFunction|CheckReady))))))

(event Custom|MCReturnToThirdPerson
  (bind _asbp_third_person_character (Utilities|Casting|CastToBP_ThirdPersonCharacter (Game|Player|GetPlayerPawn 0)))
  (Default|ReturntoThirdPerson _asbp_third_person_character))

(event Custom|RPCServerInput
  (params (Actor :type Actor%20Object%20Reference))
  (Utilities|FlowControl|Delay 2.0)
  (Actor|DestroyActor Actor))

(event EventBeginPlay
  (if (Pawn|IsLocalPlayerController)
    (CallFunction|CheckReady)))

(event Input|ActionEvents|InputActionExecuteAction
  (params (Key :type Key%20Structure :default "None"))
  (:Pressed
    (Default|CallOnInputReceived)))

(fn ConstructionScript)