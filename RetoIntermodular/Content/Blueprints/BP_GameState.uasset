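; Game state that runs the timed round loop, alternating a cannon phase with a drink game, and spawns a chest at a TriggerBox on start.
; A server-only looping one-second timer drives phase changes, and the Timer RepNotify fires an update dispatcher.
; At each day's end it prints a win if any player's score reaches 200.
; Otherwise it spawns cannons or destroys them, restoring third-person view before the drink-game countdown.
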(event Custom|EndDay
  (Utilities|Time|ClearandInvalidateTimerbyHandle (Variables|Default|GetTimerHandler))
  (for _array_element (Variables|Default|GetPlayerArray)
    (bind _asbp_player_state (Utilities|Casting|CastToBP_PlayerState _array_element))
    (if (>= (Variables|/Game/Blueprints/BP_PlayerState.BP_PlayerState_C|GetPlayerScore _asbp_player_state) 200)
      (Variables|Default|SetEndSession true)))
  (if (Variables|Default|GetEndSession)
    (Development|PrintString "You Win")
    (elif (Utilities|Enum|Equal(Enum) (Variables|Default|GetCurrentState) "NewEnumerator0")
      (Variables|Default|SetCurrentState "NewEnumerator1")
      (CallFunction|CountDowntoDrinkGame)
      (else
        (Variables|Default|SetCurrentState "NewEnumerator0")
        (CallFunction|StartTimer 1e+01 false)
        (Default|SpawnCanons (.AsBP%20Game%20Mode (Utilities|Casting|CastToBP_GameMode (Game|GetGameMode))))))))

(event Custom|StartTimer
  (params (Time :type Float%20%28double-precision%29) (Countdown :type Boolean))
  (Networking|SwitchHasAuthority
    (:Authority
      (bind _returnvalue (Utilities|Time|SetTimerbyEvent (delegate Custom|UpdateTimer) 1.0 true))
      (Variables|Default|SetTimerHandler _returnvalue))))

(event Custom|UpdateTimer
  (bind _result (Math|Float|DecrementFloat (stale Custom|StartTimer Time))
    (:%20%20
      (bind _output_get (Variables|Default|SetTimer _result))
      (if (stale Custom|StartTimer Countdown)
        (if (== _output_get 0.0)
          (Variables|Default|SetCurrentState "NewEnumerator1")
          (CallFunction|StartTimer 6e+01 false))
        (elif (== _output_get 0.0)
          (CallFunction|EndDay))))))

(event Custom|RefreshPlayers
  (Default|CallOnPlayerListChanged))

(event Custom|CountDownToDrinkGame
  (for _array_element (Variables|Default|GetPlayerArray)
    (bind _asbp_player_state (Utilities|Casting|CastToBP_PlayerState _array_element))
    (bind _asbp_player_controller (Utilities|Casting|CastToBP_PlayerController (Game|GetPlayerController _asbp_player_state)))
    (Default|MCReturntoThirdPerson _asbp_player_controller))
  (Default|DestroyCanons (.AsBP%20Game%20Mode (Utilities|Casting|CastToBP_GameMode (Game|GetGameMode))))
  (CallFunction|StartTimer 1e+01 true))

(event EventBeginPlay
  (CallFunction|StartTimer 6e+01 false)
  (bind _returnvalue (Actor|GetActorOfClass "/Script/Engine.TriggerBox"))
  (Game|SpawnActorfromClass "/Game/Blueprints/SearchChestMiniGame/BP_Chest.BP_Chest_C" (Math|Transform|MakeTransform (.location (Transformation|GetActorTransform _returnvalue)) (.rotation (Transformation|GetActorTransform _returnvalue)) "2.000000,2.000000,2.000000") "Undefined" "MultiplyWithRoot" 0 0))

(fn ConstructionScript)

(fn OnRepTimer
  (Default|CallDispatchUpdateTimer))