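; Game mode that sets up cannons for joining players and acts as an entry point for the cannon minigame.
; Each login spawns cannons at TargetPoints up to the current player count, without clearing earlier ones, then refreshes players on BP_GameState.
; StartCanonMiniGame hands off to the level's BP_CanonGameManager.
; CreateChest, CreateDrink and CreateShip wrap random-pick functions for those items.
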(event Custom|SpawnCanons
  (bind _outactors (Actor|GetAllActorsOfClass "/Script/Engine.TargetPoint"))
  (for (_array_element _array_index) _outactors
    (bind _returnvalue (Class|GameModeBase|GetNumPlayers))
    (if (< _array_index _returnvalue)
      (Game|SpawnActorfromClass "/Game/Blueprints/CanonMiniGame/BP_Canon.BP_Canon_C" (Math|Transform|MakeTransform (.location (Transformation|GetActorTransform _array_element)) (.rotation (Transformation|GetActorTransform _array_element)) "2.000000,2.000000,2.000000") "AdjustIfPossibleButDontSpawnIfColliding" "MultiplyWithRoot" 0 0))))

(event Custom|StartCanonMiniGame
  (bind _returnvalue (Actor|GetActorOfClass "/Game/Blueprints/CanonMiniGame/BP_CanonGameManager.BP_CanonGameManager_C"))
  (Default|StartMiniGame _returnvalue))

(event EventPostLogin
  (params (NewPlayer :type Player%20Controller%20Object%20Reference))
  (CallFunction|SpawnCanons)
  (bind _asbp_game_state (Utilities|Casting|CastToBP_GameState (Game|GetGameState)))
  (Default|RefreshPlayers _asbp_game_state))

(fn ConstructionScript)

(fn CreateChest
  (bind _out_row (CallFunction|GetRandomChest))
  (return _out_row))

(fn CreateDrink
  (bind _out_row (CallFunction|GetRandomDrink))
  (return _out_row))

(fn CreateShip
  (bind _randomship (CallFunction|GetRandomShip))
  (return _randomship))