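; Searchable chest actor for the chest mini-game that reveals a buff text when the nearby player gives input.
; On BeginPlay the authority gets the mesh and buff text from BP_GameMode.
; A box overlap shows a camera-facing action widget for the locally controlled character and binds the player controller's input event.
; That input swaps the widget's button for the buff text and passes the chest to the controller's server RPC.
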(event OnComponentBeginOverlap(Box)
  (params (OverlappedComponent :type Primitive%20Component%20Object%20Reference) (OtherActor :type Actor%20Object%20Reference) (OtherComp :type Primitive%20Component%20Object%20Reference) (OtherBodyIndex :type Integer) (bFromSweep :type Boolean) (SweepResult :type Hit%20Result%20Structure%20%28by%20ref%29))
  (bind _asbp_third_person_character (Utilities|Casting|CastToBP_ThirdPersonCharacter OtherActor))
  (if (Pawn|IsLocallyControlled _asbp_third_person_character)
    (Rendering|SetVisibility (Variables|Default|GetWidget) true false)
    (Variables|Default|SetPlayerInRange true)
    (EventDispatchers|BindEventtoOnInputReceived (.AsBP%20Player%20Controller (Utilities|Casting|CastToBP_PlayerController (Game|GetPlayerController 0))) (delegate Custom|ShowBuff))))

(event OnComponentEndOverlap(Box)
  (params (OverlappedComponent :type Primitive%20Component%20Object%20Reference) (OtherActor :type Actor%20Object%20Reference) (OtherComp :type Primitive%20Component%20Object%20Reference) (OtherBodyIndex :type Integer))
  (bind _asbp_third_person_character (Utilities|Casting|CastToBP_ThirdPersonCharacter OtherActor))
  (if (Pawn|IsLocallyControlled _asbp_third_person_character)
    (Rendering|SetVisibility (Variables|Default|GetWidget) false false)
    (Variables|Default|SetPlayerInRange false)))

(event Custom|ShowBuff
  (Widget|SetVisibility (Variables|/Game/Blueprints/SearchChestMiniGame/WBP_ChestAction.WBP_ChestAction_C|GetbtnExecuteAction (stale EventBeginPlay _aswbp_chest_action)) "Collapsed")
  (Rendering|Components|TextRender|SetText (Variables|/Game/Blueprints/SearchChestMiniGame/WBP_ChestAction.WBP_ChestAction_C|GettxtBuff (stale EventBeginPlay _aswbp_chest_action)) (Variables|Default|GetBuffText))
  (Widget|SetVisibility (Variables|/Game/Blueprints/SearchChestMiniGame/WBP_ChestAction.WBP_ChestAction_C|GettxtBuff (stale EventBeginPlay _aswbp_chest_action)) "Visible")
  (Default|RPCServerInput (.AsBP%20Player%20Controller (Utilities|Casting|CastToBP_PlayerController (Game|GetPlayerController 0))) self))

(event EventBeginPlay
  (bind _widget (Variables|Default|GetWidget))
  (bind _aswbp_chest_action (Utilities|Casting|CastToWBP_ChestAction (UserInterface|GetWidget _widget)))
  (Variables|/Game/Blueprints/SearchChestMiniGame/WBP_ChestAction.WBP_ChestAction_C|SetBlueprint _aswbp_chest_action self)
  (Rendering|SetVisibility _widget false false)
  (Networking|SwitchHasAuthority
    (:Authority
      (CallFunction|CreateChest))))

(event EventTick
  (params (DeltaSeconds :type Float%20%28single-precision%29))
  (Transformation|SetWorldRotation (Variables|Default|GetWidget) (Math|Rotator|FindLookatRotation (Transformation|GetWorldLocation (Variables|Default|GetWidget)) (Transformation|GetWorldLocation (Variables|/Script/Engine.PlayerCameraManager|GetTransformComponent (Game|GetPlayerCameraManager 0)))) false false))

(fn ConstructionScript)

(fn CreateChest
  (bind _returnvalue (Game|GetGameMode))
  (bind _asbp_game_mode (Utilities|Casting|CastToBP_GameMode _returnvalue))
  (Utilities|IsValid _asbp_game_mode
    (:Is%20Valid
      (bind _randomchest (Default|CreateChest _asbp_game_mode))
      (Components|StaticMesh|SetStaticMesh (Variables|Default|GetCube) (.Mesh (Utilities|Struct|BreakST_Chest _randomchest)))
      (Variables|Default|SetBuffText (.BuffText (Utilities|Struct|BreakST_Chest _randomchest))))))