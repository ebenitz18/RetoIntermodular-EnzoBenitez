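; Blueprint function library that picks random ship, chest and drink definitions from data tables.
; Each function reads all row names from DT_Ship, DT_Chest or DT_Drink, picks one at random and returns that row.
; If the row lookup fails, it only prints a not-found debug string.
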(fn GetRandomShip
  (bind _outrownames (DataTable|GetDataTableRowNames "/Game/Blueprints/Database/DT_Ship.DT_Ship"))
  (bind _returnvalue (Utilities|GetDataTableRow "/Game/Blueprints/Database/DT_Ship.DT_Ship" (.OutItem (Utilities|Array|Random _outrownames)))
    (:then
      (return _returnvalue))
    (:RowNotFound
      (Development|PrintString 0 "ShipNotFound"))))

(fn GetRandomChest
  (bind _outrownames (DataTable|GetDataTableRowNames "/Game/Blueprints/Database/DT_Chest.DT_Chest"))
  (bind _returnvalue (Utilities|GetDataTableRow "/Game/Blueprints/Database/DT_Chest.DT_Chest" (.OutItem (Utilities|Array|Random _outrownames)))
    (:then
      (return _returnvalue))
    (:RowNotFound
      (Development|PrintString 0 "ChestNotFound"))))

(fn GetRandomDrink
  (bind _outrownames (DataTable|GetDataTableRowNames "/Game/Blueprints/Database/DT_Drink.DT_Drink"))
  (bind _returnvalue (Utilities|GetDataTableRow "/Game/Blueprints/Database/DT_Drink.DT_Drink" (.OutItem (Utilities|Array|Random _outrownames)))
    (:then
      (return _returnvalue))
    (:RowNotFound
      (Development|PrintString 0 "DrinkNotFound"))))