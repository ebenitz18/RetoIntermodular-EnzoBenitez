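; BP_Canon is a player-controlled cannon for a mini-game.
; Overlapping RangeToPlay links the character to the cannon, switches its camera, hides the widget, disables the trigger and starts the Manager's mini-game.
; While in use, Tick on the locally controlled character sends control yaw and clamped pitch to ServerUpdateRotation to aim the actor.
; An externally triggered shoot event spawns BP_Bullets at the Arrow component's transform.
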(event OnComponentEndOverlap(RangeToPlay)
  (params (OverlappedComponent :type Primitive%20Component%20Object%20Reference) (OtherActor :type Actor%20Object%20Reference) (OtherComp :type Primitive%20Component%20Object%20Reference) (OtherBodyIndex :type Integer))
  (Utilities|Casting|CastToBP_ThirdPersonCharacter OtherActor)
  (Variables|Default|SetPlayerInRange false))

(event OnComponentBeginOverlap(RangeToPlay)
  (params (OverlappedComponent :type Primitive%20Component%20Object%20Reference) (OtherActor :type Actor%20Object%20Reference) (OtherComp :type Primitive%20Component%20Object%20Reference) (OtherBodyIndex :type Integer) (bFromSweep :type Boolean) (SweepResult :type Hit%20Result%20Structure%20%28by%20ref%29))
  (bind _asbp_third_person_character (Utilities|Casting|CastToBP_ThirdPersonCharacter OtherActor))
  (CallFunction|RPCSetPlayer _asbp_third_person_character)
  (Variables|Default|SetPlayerInRange true)
  (CallFunction|StartShoot)
  (Collision|SetCollisionEnabled (Variables|Default|GetRangeToPlay) "NoCollision"))

(event Custom|shoot
  (bind _arrow (Variables|Default|GetArrow))
  (bind _returnvalue (Transformation|GetWorldTransform _arrow))
  (Game|SpawnActorfromClass "/Game/Blueprints/CanonMiniGame/BP_Bullets.BP_Bullets_C" (Math|Transform|MakeTransform (.location _returnvalue) (.rotation _returnvalue) "1.000000,1.000000,1.000000") "Undefined" "MultiplyWithRoot" 0 0))

(event Custom|ServerUpdateRotation
  (params (Rotator :type Rotator))
  (Transformation|SetActorRotation self (Math|Rotator|MakeRotator (.roll Rotator) (.pitch Rotator) (.yaw Rotator))))

(event Custom|RPCSetPlayer
  (params (Character :type BP%20Third%20Person%20Character%20Object%20Reference))
  (bind _output_get (Variables|Default|SetCharacter Character))
  (Variables|/Game/Blueprints/BP_ThirdPersonCharacter.BP_ThirdPersonCharacter_C|SetCanon _output_get self))

(event Custom|StartShoot
  (bind _manager (Variables|Default|GetManager))
  (Default|ChangeCamera (Variables|Default|GetCharacter))
  (Rendering|SetVisibility (Variables|Default|GetWidget) false false)
  (Variables|Default|SetInUse true)
  (Utilities|IsValid _manager
    (:Is%20Valid
      (Default|StartMiniGame _manager))))

(event EventTick
  (params (DeltaSeconds :type Float%20%28single-precision%29))
  (bind _character (Variables|Default|GetCharacter))
  (bind _returnvalue (Pawn|GetController _character))
  (bind _returnvalue_2 (Pawn|GetControlRotation _returnvalue :!class /Script/Engine.Controller))
  (bind _returnvalue_3 (Math|Float|ClampAngle (.pitch _returnvalue_2) -5.0 45.0))
  (bind (_roll _pitch _yaw) (Math|Rotator|BreakRotator (Math|Rotator|MakeRotator 0.0 _returnvalue_3 (.yaw _returnvalue_2))))
  (Utilities|IsValid _character
    (:Is%20Valid
      (if (Pawn|IsLocallyControlled _character)
        (if (Variables|Default|GetInUse)
          (CallFunction|ServerUpdateRotation (Math|Rotator|MakeRotator _roll _pitch _yaw)))))))

(event EventBeginPlay
  (bind _aswbp_execute_action (Utilities|Casting|CastToWBP_ExecuteAction (UserInterface|GetWidget (Variables|Default|GetWidget))))
  (Variables|/Game/Blueprints/CanonMiniGame/WBP_ExecuteAction.WBP_ExecuteAction_C|SetBlueprint _aswbp_execute_action self))

(fn ConstructionScript)