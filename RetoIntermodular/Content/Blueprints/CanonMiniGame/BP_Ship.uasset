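; BP_Ship is a target ship in the cannon minigame that drifts along its local Y axis and destroys itself after ten seconds.
; Bullet overlaps on the Cube reduce Health on the authority, update the health bar through MCUpdateShipHealth and destroy the bullet.
; When Health drops below zero, the shooter's BP_PlayerState score updates and the ship is destroyed.
; Its WBP_ShipHealth widget rotates each tick to face the local player camera.
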(event OnComponentBeginOverlap(Cube)
  (params (OverlappedComponent :type Primitive%20Component%20Object%20Reference) (OtherActor :type Actor%20Object%20Reference) (OtherComp :type Primitive%20Component%20Object%20Reference) (OtherBodyIndex :type Integer) (bFromSweep :type Boolean) (SweepResult :type Hit%20Result%20Structure%20%28by%20ref%29))
  (bind _asbp_bullets (Utilities|Casting|CastToBP_Bullets OtherActor))
  (Networking|SwitchHasAuthority
    (:Authority
      (bind _output_get (Variables|Default|SetHealth (- (Variables|Default|GetHealth) 0.25)))
      (if (>= _output_get 0.0)
        (CallFunction|MCUpdateShipHealth)
        (else
          (Default|UpdateScore (.AsBP%20Player%20State (Utilities|Casting|CastToBP_PlayerState (Variables|/Script/Engine.Pawn|GetPlayerState (Variables|/Script/Engine.Actor|GetInstigator _asbp_bullets)))))
          (Actor|DestroyActor)))
      (Actor|DestroyActor _asbp_bullets))))

(event Custom|MCUpdateShipHealth
  (Default|UpdateHealth (stale EventBeginPlay _aswbp_ship_health) (stale OnComponentBeginOverlap(Cube) _output_get)))

(event EventBeginPlay
  (bind _aswbp_ship_health (Utilities|Casting|CastToWBP_ShipHealth (UserInterface|GetWidget (Variables|Default|GetWidget))))
  (Variables|/Game/Blueprints/CanonMiniGame/WBP_ShipHealth.WBP_ShipHealth_C|SetBlueprint _aswbp_ship_health self)
  (Utilities|FlowControl|Delay 1e+01)
  (Actor|DestroyActor))

(event EventTick
  (params (DeltaSeconds :type Float%20%28single-precision%29))
  (bind _widget (Variables|Default|GetWidget))
  (Transformation|AddActorLocalOffset (Math|Vector|MakeVector 0.0 (* DeltaSeconds 5e+01) 0.0) false false)
  (Transformation|SetWorldRotation _widget (Math|Rotator|FindLookatRotation (Transformation|GetWorldLocation _widget) (Camera|GetCameraLocation (Game|GetPlayerCameraManager 0))) false false))

(fn ConstructionScript)